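; Component that moves a target actor along a two-point spline segment at a set speed.
; On BeginPlay it adds a debug-drawn spline to its owner, and SetPoint places either end in world space with mirrored arrive and leave tangents.
; Move accumulates world delta time, converts it to distance via Speed, then sets the target's location and rotation from the spline.
; A helper derives travel time to the end point.
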(event `self.ReceiveBeginPlay`
  (`KismetSystemLibrary.ExecuteConsoleCommand` "show splines" null)
  (bind _returnvalue (`|AddComponentByClass` :`self` (`self.GetOwner`) :`Class` "/Script/Engine.SplineComponent"))
  (bind _output_get (set `self.Spline` _returnvalue))
  (`SplineComponent.SetUnselectedSplineSegmentColor` _output_get (`KismetMathLibrary.Conv_ColorToLinearColor` (`self.Color`)))
  (`SplineComponent.SetDrawDebug` _output_get true)
  (`SplineComponent.ClearSplinePoints` (`self.Spline`) true)
  (for _ (range 2)
    (`SplineComponent.AddSplinePoint` (`self.Spline`) (`KismetMathLibrary.Vector_Zero`) "Local" true)))

(fn `Move`
  (params (Target :type "Actor Object Reference"))
  (`self.IncrementCurrentTime`)
  (`Actor.K2_SetActorLocation` (`local.Target`) (`SplineComponent.GetLocationAtDistanceAlongSpline` (`self.Spline`) (`self.GetCurrentDistance`) "World") false false)
  (`Actor.K2_SetActorRotation` (`local.Target`) (`SplineComponent.GetRotationAtDistanceAlongSpline` (`self.Spline`) (`self.GetCurrentDistance`) "World") false))

(fn `Set Point`
  (params (Point :type "/Game/Player/Blueprints/SplineMovementByVelocity/E_SegmentPoints Enum" :default "NewEnumerator0") (InLocation :type "Vector Structure (by ref)") (InTangent :type "Vector Structure (by ref)"))
  (bind _intangent (`local.InTangent`))
  (`SplineComponent.SetLocationAtSplinePoint` (`self.Spline`) (`KismetMathLibrary.Conv_ByteToInt` Point) InLocation "World" true)
  (`SplineComponent.SetTangentsAtSplinePoint` (`self.Spline`) (`KismetMathLibrary.Conv_ByteToInt` (`local.Point`)) (`KismetMathLibrary.NegateVector` _intangent) _intangent "World" true))