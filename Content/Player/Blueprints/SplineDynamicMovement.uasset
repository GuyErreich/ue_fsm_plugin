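; Spline movement Blueprint for steering a referenced Projectile through queued target actors, then back to a return anchor.
; Tick drives an enum state machine from idle through path building, moving, retargeting and returning, with transition functions guarding state changes.
; Each leg rewrites a two-point spline using tangents from projectile orientation; segment time derives from length and Speed.
; Move and Return are empty, their movement and exit calls left unwired; Tick prints the target count.
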(event `self.ReceiveBeginPlay`)

(event `self.ReceiveTick`
  (params (DeltaSeconds :type "Float (single-precision)"))
  (`|ExecutionSequence`
    (:`then_0`
      (switch `/Game/Player/Blueprints/YonduArrow/States/E_SplineDynamicMovementStates` (`self.State`)
        (:`NewEnumerator3`
          (`self.Idle`))
        (:`NewEnumerator4`
          (`self.Build Path`))
        (:`NewEnumerator0`
          (`self.Move`))
        (:`NewEnumerator6`
          (`self.Finished Moving`))
        (:`NewEnumerator5`
          (`self.Set Next Target`))
        (:`NewEnumerator1`
          (`self.Set Return Path`))
        (:`NewEnumerator7`
          (`self.Return`))))
    (:`then_1`
      (`KismetSystemLibrary.PrintString` (`KismetStringLibrary.Conv_IntToString` (`KismetArrayLibrary.Array_Length` (`self.Targets`)))))))

(event `Idle`
  (`self.Idle -> Build Path`))

(event `Build Path`
  (`self.CreateStartingSegment`)
  (`self.Build Path -> Move`))

(event `Move`)

(event `Finished Moving`
  (`self.StopMoving`)
  (`self.Remove Current Target`)
  (`self.FInished Moving -> Set Next Target`)
  (`self.FInished Moving -> Set Return Path`))

(event `Set Next Target`
  (`self.Retarget`)
  (`self.Set Next Target -> Move`))

(event `Set Return Path`
  (`self.Add Target` (`self.ReturnPointAnchor`))
  (`self.Retarget`)
  (`self.Set Return Path -> Return`))

(event `Return`)

(fn `Add Target`
  (params (Target :type "Actor Object Reference (by ref)"))
  (bind _targets (`self.Targets`))
  (if (not (== (`|GetArrayItem` _targets (`KismetArrayLibrary.Array_LastIndex` _targets)) (`local.Target`)))
    (`KismetArrayLibrary.Array_Add` (`self.Targets`) (`local.Target`))))

(fn `Build Path -> Move`
  (set `self.State` "NewEnumerator0"))

(fn `Clear Targets`
  (`KismetArrayLibrary.Array_Clear` (`self.Targets`)))

(fn `CreateStartingSegment`
  (bind _projectile (`self.Projectile`))
  (set `self.Tangent Location` (`self.CalculateTangent` (`self.StartPoint`) (+ (`self.GetActorForwardVector` _projectile) (`self.GetActorRightVector` _projectile))))
  (`self.Update Segment` (`self.K2_GetActorLocation` (`self.Projectile`)) (`self.Tangent Location`) (`self.GetCurrentTargetPosition`) (`KismetMathLibrary.NegateVector` (`self.Tangent Location`)) (`self.Tangent Location`)))

(fn `FInished Moving -> Set Next Target`
  (if (`KismetArrayLibrary.Array_IsNotEmpty` (`self.Targets`))
    (set `self.State` "NewEnumerator5")))

(fn `FInished Moving -> Set Return Path`
  (if (`KismetArrayLibrary.Array_IsEmpty` (`self.Targets`))
    (set `self.State` "NewEnumerator1")))

(fn `Idle -> Build Path`
  (if (`KismetArrayLibrary.Array_IsNotEmpty` (`self.Targets`))
    (set `self.State` "NewEnumerator4")))

(fn `InitializeActorReferences`
  (params (Projectile :type "Actor Object Reference") (ReturnPointAnchor :type "Actor Object Reference"))
  (set `self.Projectile` Projectile)
  (set `self.ReturnPointAnchor` ReturnPointAnchor))

(fn `Move -> Finished Moving`
  (if (> (`self.CurrentTime`) (`self.GetTimeOfCurrentSegment`))
    (set `self.State` "NewEnumerator6")))

(fn `Remove Current Target`
  (`KismetArrayLibrary.Array_Remove` (`self.Targets`)))

(fn `Retarget`
  (set `self.Tangent Location` (`self.CalculateTangent` (`self.GetCurrentTargetPosition`) (`self.GetActorForwardVector` (`self.Projectile`))))
  (`self.Update Segment` (`self.K2_GetActorLocation` (`self.Projectile`)) (`self.Tangent Location`) (`self.GetCurrentTargetPosition`) (`KismetMathLibrary.NegateVector` (`self.Tangent Location`)) (`self.Tangent Location`)))

(fn `Return -> Idle`
  (if (> (`self.CurrentTime`) (`self.GetTimeOfCurrentSegment`))
    (`self.Remove Current Target`)
    (set `self.State` "NewEnumerator3")))

(fn `Set Next Target -> Move`
  (set `self.State` "NewEnumerator0"))

(fn `Set Return Path -> Return`
  (set `self.State` "NewEnumerator7"))

(fn `StopMoving`
  (set `self.CurrentTime` 0.0))

(fn `Update Segment`
  (params (`Start Point` :type "Vector Structure (by ref)") (`Start Point Tangent` :type "Vector Structure (by ref)") (`End Point` :type "Vector Structure (by ref)") (`End Point Arrive Tangent` :type "Vector Structure (by ref)") (`End Point Leave Tangent` :type "Vector Structure (by ref)"))
  (`SplineComponent.SetLocationAtSplinePoint` (`self.Spline`) 0 `Start Point` "World" true)
  (`SplineComponent.SetTangentAtSplinePoint` (`self.Spline`) 0 `Start Point Tangent` "World" true)
  (`SplineComponent.SetLocationAtSplinePoint` (`self.Spline`) 1 `End Point` "World" true)
  (`SplineComponent.SetTangentsAtSplinePoint` (`self.Spline`) 1 `End Point Arrive Tangent` `End Point Leave Tangent` "World" true))

(fn `Update Target Point Position`
  (`SplineComponent.SetLocationAtSplinePoint` (`self.Spline`) 1 (`self.GetCurrentTargetPosition`) "World" true))

(fn `UserConstructionScript`
  (`SplineComponent.ClearSplinePoints` (`self.Spline`) true)
  (`SplineComponent.AddPoint` (`self.Spline`) (make `SplinePoint` 0.0) true)
  (`SplineComponent.AddPoint` (`self.Spline`) (make `SplinePoint` 1.0) true))