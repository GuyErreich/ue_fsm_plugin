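; Movement component for the player's Yondu arrow that flies its owning actor along a curved spline to a target component.
; Setting a target shapes a runtime spline using a configurable launch direction and curve strength, optionally aligning arrival with the target's forward vector to hit from behind.
; Each tick pins the endpoint to the moving target, advances normalized time, applies the spline transform, and clears the target on completion.
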(event `self.ReceiveBeginPlay`
  (bind _returnvalue (`|AddComponentByClass` (`self.GetOwner`) "/Script/Engine.SplineComponent" true (`KismetMathLibrary.MakeTransform` (0.0 0.0 0.0))))
  (bind _output_get (set `self.Spline` _returnvalue))
  (`SplineComponent.SetDrawDebug` _output_get true)
  (`SplineComponent.SetSplinePoints` (`self.Spline`) (`self.Points`) "World" true))

(event `self.ReceiveTick`
  (params (DeltaSeconds :type "Float (single-precision)"))
  (`|ExecutionSequence`
    (:`then_0`
      (`self.Update Target Position`))
    (:`then_1`
      (if (`KismetSystemLibrary.IsValid` (`self.Target`))
        (set `self.Is Moving` true)
        (`self.Move`)))
    (:`then_2`
      (if (>= (`self.Time`) 1.0)
        (set `self.Is Moving` false)
        (`self.Set Target` null)
        (set `self.Time` 0.0)))))

(fn `Create Spline`
  (locals (NewLocalVar :type "Vector Structure" :default (0.0 0.0 0.0)) (NewLocalVar_0 :type "Vector Structure" :default (0.0 0.0 0.0)))
  (bind _returnvalue (`self.GetOwner`))
  (`|ExecutionSequence`
    (:`then_0`
      (`SplineComponent.SetLocationAtSplinePoint` (`self.Spline`) 0 (`Actor.K2_GetActorLocation` (`self.GetOwner`)) "World" true)
      (`SplineComponent.SetTangentAtSplinePoint` (`self.Spline`) 0 (* (`KismetMathLibrary.Normal` (+ (* (`Actor.GetActorForwardVector` _returnvalue) (.x (`self.Direction`))) (* (`Actor.GetActorRightVector` _returnvalue) (.y (`self.Direction`))) (* (`Actor.GetActorUpVector` _returnvalue) (.z (`self.Direction`))))) (`self.Curve Strength`)) "Local" true)
      (if (`self.Hit From Back`)
        (`SplineComponent.SetTangentAtSplinePoint` (`self.Spline`) 1 (* (`SceneComponent.GetForwardVector` (`self.Target`)) (`self.Curve Strength`)) "Local" true)
        (else
          (`SplineComponent.SetSplinePointType` (`self.Spline`) 1 "Constant" true))))))

(fn `Get Position`
  (returns (ReturnValue :type "Transform Structure"))
  (bind (_returnvalue_location _returnvalue_rotation) (`KismetMathLibrary.BreakTransform` (`SplineComponent.GetTransformAtTime` (`self.Spline`) (`self.Time`) "World" false true)))
  (return (`KismetMathLibrary.MakeTransform` _returnvalue_location _returnvalue_rotation (`Actor.GetActorScale3D` (`self.GetOwner`)))))

(fn `Move`
  (locals (`Target Position` :type "Transform Structure"))
  (set `self.Time` (+ (/ (`GameplayStatics.GetWorldDeltaSeconds`) (`self.Total Time Across Distance`)) (`self.Time`)))
  (bind _returnvalue (`self.Get Position`))
  (set `local.Target Position` _returnvalue)
  (`SceneComponent.K2_SetWorldTransform` (`Actor.RootComponent` (`self.GetOwner`)) (`local.Target Position`) false false))

(fn `Set Target`
  (params (Target :type "SceneComponent Object Reference"))
  (set `self.Target` Target)
  (set `self.Time` 0.0)
  (`self.Create Spline`))

(fn `Update Target Position`
  (bind _target (`self.Target`))
  (`/Engine/EditorBlueprintResources/StandardMacros.IsValid` _target
    (:`Is Valid`
      (`SplineComponent.SetLocationAtSplinePoint` (`self.Spline`) 1 (`SceneComponent.K2_GetComponentLocation` _target) "World" true))))