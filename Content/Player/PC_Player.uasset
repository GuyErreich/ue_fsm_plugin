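; PC_Player is a player controller Blueprint that turns Enhanced Input actions into movement and look for the pawn it controls.
; BeginPlay adds the mapping context and caches the controlled pawn.
; IA_Movement moves the cached pawn along right and forward vectors built from control-rotation yaw only, so pitch does not affect direction.
; IA_Look fetches the controlled pawn on each event and adds yaw and pitch input.
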(event `self.ReceiveBeginPlay`
  (`EnhancedInputSubsystemInterface.AddMappingContext` (pcsubsystem `EnhancedInputLocalPlayerSubsystem` self) (`self.Mapping Context`) 0 (struct))
  (set `self.Controlled Pawn` (`self.K2_GetPawn`)))

(event `EnhancedInput|/Game/Player/Input/Actions/IA_Movement`
  (params (ActionValue :type "Vector2D Structure") (ElapsedSeconds :type "Float (double-precision)") (TriggeredSeconds :type "Float (double-precision)") (InputAction :type "InputAction Object Reference" :default "/Game/Player/Input/Actions/IA_Movement.IA_Movement"))
  (bind (_returnvalue_roll _returnvalue_pitch _returnvalue_yaw) (`KismetMathLibrary.BreakRotator` (`self.GetControlRotation`)))
  (bind (_returnvalue_roll_2 _returnvalue_pitch_2 _returnvalue_yaw_2) (`KismetMathLibrary.BreakRotator` (`self.GetControlRotation`)))
  ;[1 1 1] Movement
  (:`Triggered`
    (`Pawn.AddMovementInput` (`self.Controlled Pawn`) (`KismetMathLibrary.GetRightVector` (`KismetMathLibrary.MakeRotator` 0.0 0.0 _returnvalue_yaw_2)) ActionValue_X false)
    (`Pawn.AddMovementInput` (`self.Controlled Pawn`) (`KismetMathLibrary.GetForwardVector` (`KismetMathLibrary.MakeRotator` 0.0 0.0 _returnvalue_yaw)) ActionValue_Y false)))

(event `EnhancedInput|/Game/Player/Input/Actions/IA_Look`
  (params (ActionValue :type "Vector2D Structure") (ElapsedSeconds :type "Float (double-precision)") (TriggeredSeconds :type "Float (double-precision)") (InputAction :type "InputAction Object Reference" :default "/Game/Player/Input/Actions/IA_Look.IA_Look"))
  (bind _returnvalue (`self.K2_GetPawn`))
  ;[1 1 1] Look
  (:`Triggered`
    (`Pawn.AddControllerYawInput` _returnvalue ActionValue_X)
    (`Pawn.AddControllerPitchInput` _returnvalue ActionValue_Y)))

(fn `UserConstructionScript`)